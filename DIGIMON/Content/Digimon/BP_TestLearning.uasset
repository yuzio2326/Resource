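; Test Learning Agents actor that, on BeginPlay, registers itself with the LearningAgentsManager on actors tagged "TestLearningAgentManager".
; TraceRotate line-traces on the Camera channel and reports whether the hit actor's first tag is Alpha or Beta.
; ShouldShoot repeats the trace, returning an Alpha flag and the hit actor.
; Both compute the trace end by dividing location by scaled forward vector, rather than adding it.
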(event `self.ReceiveBeginPlay`
  (`|ExecutionSequence`
    (:`then_0`
      (bind _outactors (`GameplayStatics.GetAllActorsWithTag` "TestLearningAgentManager"))
      (for _array_element _outactors
        (bind _returnvalue (`self.GetComponentByClass` _array_element "/Script/LearningAgents.LearningAgentsManager"))
        (`/Engine/EditorBlueprintResources/StandardMacros.IsValid` _returnvalue
          (:`Is Valid`
            (`LearningAgentsManager.AddAgent` _returnvalue self)))))))

(event `self.ReceiveActorBeginOverlap`
  (params (OtherActor :type "Actor Object Reference")))

(fn `ShouldShoot`
  (returns (HitTeamAlpha1 :type Boolean) (HitActor :type "Actor Object Reference"))
  (locals (HitTeamAlpha :type Boolean))
  (bind _returnvalue (`self.K2_GetActorLocation`))
  (set `local.HitTeamAlpha` false)
  (bind (_outhit _returnvalue_2) (`KismetSystemLibrary.LineTraceSingle` _returnvalue (/ _returnvalue (* (`self.GetActorForwardVector`) 1000.0)) "TraceTypeQuery2"))
  (if _returnvalue_2
    (bind (_bblockinghit _binitialoverlap _time _distance _location _impactpoint _normal _impactnormal _physmat _hitactor) (`GameplayStatics.BreakHitResult` _outhit))
    (bind _tags (`Actor.Tags` _hitactor))
    (if (`KismetArrayLibrary.Array_IsEmpty` _tags)
      (set `local.HitTeamAlpha` false)
      (else
        (set `local.HitTeamAlpha` (== (`|GetArrayItem` _tags) "Alpha"))))
    (else
      (set `local.HitTeamAlpha` false)))
  (return (`local.HitTeamAlpha`) _hitactor))

(fn `TraceRotate`
  (returns (HitTeamAlpha1 :type Boolean) (HitTeamBeta1 :type Boolean))
  (locals (HitTeamAlpha :type Boolean) (HitTeamBeta :type Boolean))
  (bind _returnvalue (`self.K2_GetActorLocation`))
  (set `local.HitTeamBeta` false)
  (set `local.HitTeamAlpha` false)
  (bind (_outhit _returnvalue_2) (`KismetSystemLibrary.LineTraceSingle` _returnvalue (/ _returnvalue (* (`self.GetActorForwardVector`) 1000.0)) "TraceTypeQuery2"))
  (if _returnvalue_2
    (bind _tags (`Actor.Tags` (`.HitActor` (`GameplayStatics.BreakHitResult` _outhit))))
    (if (`KismetArrayLibrary.Array_IsEmpty` _tags)
      (set `local.HitTeamBeta` false)
      (set `local.HitTeamAlpha` false)
      (else
        (set `local.HitTeamAlpha` (== (`|GetArrayItem` _tags) "Alpha"))
        (set `local.HitTeamBeta` (== (`|GetArrayItem` _tags) "Beta"))))
    (else
      (set `local.HitTeamBeta` false)
      (set `local.HitTeamAlpha` false)))
  (return (`local.HitTeamAlpha`) (`local.HitTeamBeta`)))

(fn `UserConstructionScript`)